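; TestDamage is a test actor that applies a fixed amount of damage to any actor that begins overlapping its box, naming itself as the causer.
; A take-any-damage handler casts the damage type to NewBlueprint and switches on its Damage or Heal enum, printing the same placeholder text for both.
; The node that binds this handler is never executed, so this graph does not hook it up.
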(event OnComponentBeginOverlap(Box)
  (params (OverlappedComponent :type Primitive%20Component%20Object%20Reference) (OtherActor :type Actor%20Object%20Reference) (OtherComp :type Primitive%20Component%20Object%20Reference) (OtherBodyIndex :type Integer) (bFromSweep :type Boolean) (SweepResult :type Hit%20Result%20Structure%20%28by%20ref%29))
  (Game|Damage|ApplyDamage OtherActor 1e+01 0 self (Variables|Default|GetDamage%20Type%20Class)))

(event Custom|OnTakeAnyDamage_Event
  (params (DamagedActor :type Actor%20Object%20Reference) (Damage :type Float%20%28single-precision%29) (DamageType :type Damage%20Type%20Object%20Reference) (InstigatedBy :type Controller%20Object%20Reference) (DamageCauser :type Actor%20Object%20Reference))
  (bind (_asnew_blueprint _bsuccess) (Utilities|Casting|CastToNewBlueprint DamageType))
  (if _bsuccess
    (switch Utilities|FlowControl|Switch|SwitchonDamage (Variables|/Game/Blueprint/NewBlueprint.NewBlueprint_C|GetNewVar _asnew_blueprint)
      (:NewEnumerator0
        (Development|PrintString "Hello"))
      (:NewEnumerator1
        (Development|PrintString "Hello")))))

(event EventBeginPlay)

(event Collision|EventActorBeginOverlap
  (params (OtherActor :type Actor%20Object%20Reference)))

(event EventTick
  (params (DeltaSeconds :type Float%20%28single-precision%29)))

(fn ConstructionScript)