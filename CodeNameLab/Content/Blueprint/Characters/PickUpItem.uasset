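; PickUpItem lets its owner pick up and place items by destroying and respawning actors.
; Key 1 line-traces forward from the owner on the Visibility channel, stores the hit actor's class and destroys that actor.
; Key 2 spawns a fresh instance of the stored class at the trace's full distance ahead, using the owner's rotation and scale.
; Only the class is kept, so instance state is lost.
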(event EventBeginPlay)

(event EventTick
  (params (DeltaSeconds :type Float%20%28single-precision%29)))

(event Input|KeyboardEvents|1
  (params (Key :type Key%20Structure :default "None"))
  (bind _returnvalue (Components|GetOwner))
  (bind _returnvalue_2 (Transformation|GetActorLocation _returnvalue))
  (:Pressed
    (bind (_outhit _returnvalue_3) (Collision|LineTraceByChannel _returnvalue_2 (+ _returnvalue_2 (* (Transformation|GetActorForwardVector _returnvalue) 1e+03)) "TraceTypeQuery1" false 0 "None"))
    (if _returnvalue_3
      (Variables|Default|SetHit%20Actor (Utilities|GetClass (.HitActor (Collision|BreakHitResult _outhit))))
      (Actor|DestroyActor (.HitActor (Collision|BreakHitResult _outhit))))))

(event Input|KeyboardEvents|2
  (params (Key :type Key%20Structure :default "None"))
  (bind _returnvalue (Components|GetOwner))
  (bind _returnvalue_2 (Transformation|GetActorTransform _returnvalue))
  (:Pressed
    (Game|SpawnActorfromClass (Variables|Default|GetHit%20Actor) (Math|Transform|MakeTransform (+ (.location _returnvalue_2) (* (Transformation|GetActorForwardVector _returnvalue) 1e+03)) (.rotation _returnvalue_2) (.scale _returnvalue_2)) "Undefined" "MultiplyWithRoot" 0 0)))